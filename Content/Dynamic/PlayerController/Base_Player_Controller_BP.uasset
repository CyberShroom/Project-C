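; Base player controller that drives an Entity_Ship pawn's forward/backward movement and yaw from Enhanced Input, in singleplayer or networked play.
; Input applies movement locally and sends it by server RPC, which reapplies it only for non-local controllers so the host does not move twice.
; Turning counter-rotates the ship's camera, found by casting the pawn to Entity_Ship.
; On BeginPlay the authority resets player 0's pawn to the origin, and local players add Basic_Controls.
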(event `EnhancedInput|/Game/Dynamic/KeyMapping/BasicControls/Move_Vertical`
  (params (ActionValue :type "Float (double-precision)") (ElapsedSeconds :type "Float (double-precision)") (TriggeredSeconds :type "Float (double-precision)") (InputAction :type "InputAction Object Reference" :default "/Game/Dynamic/KeyMapping/BasicControls/Move_Vertical.Move_Vertical"))
  ;[1 1 1] Allows Pawn to move forward and backward
  (:`Triggered`
    (`self.SERVERRPC-InputVertical` ActionValue)
    (`self.MovePawn` ActionValue)))

(event `SERVERRPC-InputVertical`
  (params (Value :type "Float (double-precision)"))
  ;[1 1 1] Allows Pawn to move forward and backward
  (if (not (`self.IsLocalPlayerController` self))
    (`self.MovePawn` Value)))

(event `EnhancedInput|/Game/Dynamic/KeyMapping/BasicControls/Turn`
  (params (ActionValue :type "Float (double-precision)") (ElapsedSeconds :type "Float (double-precision)") (TriggeredSeconds :type "Float (double-precision)") (InputAction :type "InputAction Object Reference" :default "/Game/Dynamic/KeyMapping/BasicControls/Turn.Turn"))
  ;[1 1 1] BOTH: Allows pawn to turn left and right. The Camera recieves inverse rotation.
  (:`Triggered`
    (`self.SERVERRPC-InputTurn` ActionValue)
    (`self.TurnPawn` ActionValue)))

(event `SERVERRPC-InputTurn`
  (params (Value :type "Float (double-precision)"))
  ;[1 1 1] BOTH: Allows pawn to turn left and right. The Camera recieves inverse rotation.
  (if (not (`self.IsLocalPlayerController` self))
    (`self.TurnPawn` Value)))

(event `self.ReceiveBeginPlay`
  ;[1 1 1] The Server sets the player pawn location. The Client sets up its Input Context. Server runs SetEIContext for the host pawn and singleplayer.
  (`/Engine/EditorBlueprintResources/ActorMacros.Switch Has Authority`
    (:`Authority`
      (`self.SetPawnLocation`)
      (if (`self.IsLocalPlayerController` self)
        (`self.SetEIContext`)))
    (:`Remote`
      (`self.SetEIContext`))))

(fn `GetPawnCamera`
  (returns (Camera :type "CameraComponent Object Reference"))
  (bind _asentity_ship (cast `/Game/Dynamic/Classes/Entity_Ship/Entity_Ship` (`self.K2_GetPawn`))
    (:`then`
      _)
    (:`CastFailed`
      (`KismetSystemLibrary.PrintString` "SEVERE: Could not find a Camera on the player pawn! Did you change the subclass? The player pawn must be a subclass of Entity_Ship! Please Close the game, it will not run properly!" true true (struct :`R` 1.0 :`A` 1.0) 10.0)))
  (return (`/Game/Dynamic/Classes/Entity_Ship/Entity_Ship.Camera` _asentity_ship)))

(fn `MovePawn`
  (params (moveSpeed :type "Float (double-precision)"))
  (`self.K2_AddActorLocalOffset` (`self.K2_GetPawn`) (`KismetMathLibrary.MakeVector` (* moveSpeed (`self.moveSpeed`))) false false))

(fn `SetEIContext`
  (`EnhancedInputSubsystemInterface.AddMappingContext` (pcsubsystem `EnhancedInputLocalPlayerSubsystem` self) "/Game/Dynamic/KeyMapping/BasicControls/Basic_Controls.Basic_Controls" 0 (struct)))

(fn `SetPawnLocation`
  (`self.K2_SetActorLocation` (`GameplayStatics.GetPlayerPawn` 0) (0.0 0.0 0.0) false false))

(fn `TurnPawn`
  (params (turnSpeed :type "Float (double-precision)"))
  (bind _returnvalue (* turnSpeed (`self.turnSpeed`)))
  (`self.K2_AddActorLocalRotation` (`self.K2_GetPawn`) (`KismetMathLibrary.MakeRotator` 0.0 0.0 _returnvalue) false false)
  (bind _camera (`self.GetPawnCamera`))
  (bind _result (`/Engine/EditorBlueprintResources/StandardMacros.NegateFloat` _returnvalue)
    (:`  `
      (`SceneComponent.K2_AddRelativeRotation` _camera (`KismetMathLibrary.MakeRotator` 0.0 0.0 _result) false false))))

(fn `UpdateMoveSpeed`
  (params (newSpeed :type "Float (double-precision)"))
  (set `self.moveSpeed` newSpeed))

(fn `UpdateTurnSpeed`
  (params (newSpeed :type "Float (double-precision)"))
  (set `self.turnSpeed` newSpeed))

(fn `UserConstructionScript`)